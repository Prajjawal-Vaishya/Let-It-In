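; BP_Ghost is an AI enemy that detects the player and makes melee attacks.
; Pawn sensing sets the seeingPlayer Blackboard key for Player-tagged pawns, and a retriggerable delay clears it a few seconds after the last sighting of any pawn.
; The Attack event plays a zombie montage, guarded against re-entry until completion, and immediately sphere-traces forward from AttackTrackPoint to damage a hit pawn.
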(event OnSeePawn(PawnSensing)
  (params (Pawn :type Pawn%20Object%20Reference))
  (bind _returnvalue (Utilities|Name|MakeLiteralName "seeingPlayer"))
  (bind _self self)
  (bind _returnvalue_2 (AI|GetAIController _self))
  (bind _returnvalue_3 (AI|GetBlackboard _returnvalue_2))
  (Utilities|FlowControl|Sequence
    (:then_0
      (if (Actor|ActorHasTag Pawn "Player")
        (AI|Components|Blackboard|SetValueasBool _returnvalue_3 _returnvalue true)))
    (:then_1
      (Utilities|FlowControl|RetriggerableDelay 3.0)
      (AI|Components|Blackboard|SetValueasBool _returnvalue_3 _returnvalue false))))

(event Custom|Attack
  (bind _attack_track_point (Variables|Default|GetAttack%20Track%20Point))
  (bind _returnvalue (Transformation|GetWorldLocation _attack_track_point))
  (if (not (Variables|Default|Getattack?))
    (Variables|Default|Setattack? true)
    (Animation|Montage|PlayMontage (Variables|Character|GetMesh) "/Game/AIGhost/AI_Character/Zombie_Attack_Montage.Zombie_Attack_Montage"
      (:then
        (bind (_outhit _returnvalue_2) (Collision|SphereTraceForObjects _returnvalue (+ _returnvalue (* (Math|Vector|GetForwardVector (Transformation|GetWorldRotation _attack_track_point)) 7e+01)) 25.0 (Utilities|Array|MakeArray "ObjectTypeQuery3") false 0 "None"))
        (if _returnvalue_2
          (Game|Damage|ApplyDamage (.HitActor (Collision|BreakHitResult _outhit)) 2e+01 0 self)))
      (:OnCompleted
        (Variables|Default|Setattack? false)))))

(event Collision|EventActorBeginOverlap
  (params (OtherActor :type Actor%20Object%20Reference)))

(event EventTick
  (params (DeltaSeconds :type Float%20%28single-precision%29)))

(fn ConstructionScript)