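; Enterable drawer that the player gets in and out of through the Interact event.
; Each interaction flips an Inside flag, teleports player 0 to the REFIn or REFOut marker transform, and snaps the Door shut on entry or open on exit.
; A Trigger overlap prints a debug key hint, while Box overlaps with Player-tagged actors call EnterOverlap and ExitOverlap.
; The interaction prompt and CanInteract functions are stubs returning false.
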(event OnComponentBeginOverlap(Trigger)
  (params (OverlappedComponent :type Primitive%20Component%20Object%20Reference) (OtherActor :type Actor%20Object%20Reference) (OtherComp :type Primitive%20Component%20Object%20Reference) (OtherBodyIndex :type Integer) (bFromSweep :type Boolean) (SweepResult :type Hit%20Result%20Structure%20%28by%20ref%29))
  (Utilities|Casting|CastToBP_Player OtherActor)
  (Development|PrintString "Press E to get inside"))

(event OnComponentBeginOverlap(Box)
  (params (OverlappedComponent :type Primitive%20Component%20Object%20Reference) (OtherActor :type Actor%20Object%20Reference) (OtherComp :type Primitive%20Component%20Object%20Reference) (OtherBodyIndex :type Integer) (bFromSweep :type Boolean) (SweepResult :type Hit%20Result%20Structure%20%28by%20ref%29))
  (if (Actor|ActorHasTag OtherActor "Player")
    (CallFunction|EnterOverlap)))

(event OnComponentEndOverlap(Box)
  (params (OverlappedComponent :type Primitive%20Component%20Object%20Reference) (OtherActor :type Actor%20Object%20Reference) (OtherComp :type Primitive%20Component%20Object%20Reference) (OtherBodyIndex :type Integer))
  (if (Actor|ActorHasTag OtherActor "Player")
    (CallFunction|ExitOverlap)))

(event EventBeginPlay)

(event EventInteract
  (bind _ref_in (Variables|Default|GetREF%20in))
  (bind _ref_out (Variables|Default|GetREF%20out))
  (bind _returnvalue (Transformation|GetWorldTransform _ref_in))
  (bind _returnvalue_2 (Transformation|GetWorldTransform _ref_out))
  (if (not (Variables|Default|Getinside))
    (Variables|Default|Setinside true)
    (Transformation|SetActorTransform (Game|GetPlayerCharacter 0) (Math|Transform|MakeTransform (.location _returnvalue) (.rotation _returnvalue) (.scale _returnvalue)))
    (Transformation|SetRelativeRotation (Variables|Default|GetDoor) "0, 0, 0" false false)
    (else
      (Variables|Default|Setinside false)
      (Transformation|SetActorTransform (Game|GetPlayerCharacter 0) (Math|Transform|MakeTransform (.location _returnvalue_2) (.rotation _returnvalue_2) (.scale _returnvalue_2)))
      (Transformation|SetRelativeRotation (Variables|Default|GetDoor) "0.000000,109.999999,0.000000" false false))))

(fn ConstructionScript)

(fn InteractPrompt
  (return false "None"))

(fn CanInteract?
  (return false))