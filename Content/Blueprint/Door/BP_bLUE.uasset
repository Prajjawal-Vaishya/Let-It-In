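; Door actor that swings open when an actor tagged "Ghost" enters its Box trigger.
; The overlap plays the TL_Door timeline, whose Alpha lerps the Door's absolute world yaw from 0 to 90 degrees.
; End overlap checks the same tag but does nothing, so the door has no closing logic.
; A Gate and FlipFlop chain into the timeline is left unconnected and never runs.
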(event OnComponentBeginOverlap(Box)
  (params (OverlappedComponent :type Primitive%20Component%20Object%20Reference) (OtherActor :type Actor%20Object%20Reference) (OtherComp :type Primitive%20Component%20Object%20Reference) (OtherBodyIndex :type Integer) (bFromSweep :type Boolean) (SweepResult :type Hit%20Result%20Structure%20%28by%20ref%29))
  (if (Actor|ActorHasTag OtherActor "Ghost")
    (bind _alpha (Timeline|TL_Door Play)
      (:Update
        (Transformation|SetWorldRotation (Variables|Default|GetDoor) (Math|Rotator|MakeRotator 0.0 0.0 (Math|Float|Lerp 0.0 9e+01 _alpha)) false false)))))

(event OnComponentEndOverlap(Box)
  (params (OverlappedComponent :type Primitive%20Component%20Object%20Reference) (OtherActor :type Actor%20Object%20Reference) (OtherComp :type Primitive%20Component%20Object%20Reference) (OtherBodyIndex :type Integer))
  (if (Actor|ActorHasTag OtherActor "Ghost")
    _))

(fn ConstructionScript)