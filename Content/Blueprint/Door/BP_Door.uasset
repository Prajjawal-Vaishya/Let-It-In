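; Door that swings open or closed each time an actor tagged Ghost enters its box, and stays locked to interacting players.
; A timeline drives the yaw forward or in reverse, triggering the open or close sound near the shut angle.
; Interact only shows an unlock notification, plays a try-open sound and nudges the door, with no key check.
; The interaction queries always return false, and several older jiggle and opening chains sit disconnected.
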(event OnComponentBeginOverlap(Box)
  (params (OverlappedComponent :type Primitive%20Component%20Object%20Reference) (OtherActor :type Actor%20Object%20Reference) (OtherComp :type Primitive%20Component%20Object%20Reference) (OtherBodyIndex :type Integer) (bFromSweep :type Boolean) (SweepResult :type Hit%20Result%20Structure%20%28by%20ref%29))
  (if (Actor|ActorHasTag OtherActor "Ghost")
    (Variables|Default|SetCanInteract? false)
    (if (Variables|Default|GetIsClosed)
      (Variables|Default|SetIsClosed false)
      (bind _alpha (Timeline|Timeline_0 PlayFromStart)
        (:Update
          (Transformation|SetRelativeRotation (Variables|Default|GetDoor) (Math|Rotator|MakeRotator 0.0 0.0 (Math|Float|Lerp 0.0 (Variables|Default|GetOpenDegrees) _alpha)) false false)
          (Utilities|FlowControl|Sequence
            (:then_0
              (if (or (Math|Float|NearlyEqual(Float) (Math|Float|Lerp 0.0 (Variables|Default|GetOpenDegrees) _alpha) 2.0 2.0) (Math|Float|NearlyEqual(Float) (Math|Float|Lerp 0.0 (Variables|Default|GetOpenDegrees) _alpha) -2.0 2.0))
                (Utilities|FlowControl|DoOnce false :!label _label
                  (:Completed
                    (Audio|PlaySoundatLocation (select (Variables|Default|GetIsClosed) (Variables|Default|GetCloseSound) (Variables|Default|GetOpenSound)) (Transformation|GetActorLocation) "0, 0, 0" 0.5 1.0 0.0 "/Game/FPMovement/Assets/Audio/Abilitys/Door/Effects/DoorAttenuation.DoorAttenuation" 0 0 0)))))
            (:then_1
              (if true
                (goto _label Reset)))))
        (:Finished
          (Variables|Default|SetCanInteract? true)
          (goto _label Reset)))
      (else
        (Variables|Default|SetIsClosed true)
        (Timeline|Timeline_0 ReverseFromEnd)))))

(event OnComponentEndOverlap(Box)
  (params (OverlappedComponent :type Primitive%20Component%20Object%20Reference) (OtherActor :type Actor%20Object%20Reference) (OtherComp :type Primitive%20Component%20Object%20Reference) (OtherBodyIndex :type Integer)))

(event EventInteract
  (params (Player :type BP%20Player%20Object%20Reference))
  (Default|AddNotification (Variables|/Game/FPMovement/Player/Blueprints/BP_Player.BP_Player_C|GetWP_PlayerHUD Player) (Variables|Default|GetUnlock%20Notification) (Variables|Default|GetDoor%20Name%20Notification) (Variables|Default|GetDoor%20Name%20Color%20Notification))
  (Audio|PlaySoundatLocation (Variables|Default|GetTryOpenSound) (Transformation|GetActorLocation) "0, 0, 0" 0.5 1.0 0.0 "/Game/FPMovement/Assets/Audio/Abilitys/Door/Effects/DoorAttenuation.DoorAttenuation" 0 0 0)
  (Development|PrintString "No key or wrong key" true true "(R=0.000000,G=0.660000,B=1.000000,A=1.000000)" 2.0 "")
  (bind _alpha (Timeline|Timeline_1 PlayFromStart)
    (:Update
      (Transformation|SetRelativeRotation (Variables|Default|GetDoor) (Math|Rotator|MakeRotator 0.0 0.0 (Math|Float|Lerp 0.0 0.4 _alpha)) false false))))

(fn ConstructionScript)

(fn CanInteract?
  (return false))

(fn InteractPrompt
  (return false "None"))