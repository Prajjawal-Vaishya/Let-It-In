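; BP_ParentDropItem is a base Blueprint for drop items that alerts the BP_Ghost AI to a noise.
; On BeginPlay it caches a reference to the BP_Ghost found in the level.
; Its AICall event writes the hit location to the ghost's NoiseLocation Blackboard key, then pulses soundPlay from false to true across a short delay and prints a debug message.
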(event Custom|AICall
  (params (HitLocation :type Vector))
  (bind _ghostref (Variables|Default|GetGhostRef))
  (bind _returnvalue (AI|GetAIController _ghostref))
  (bind _returnvalue_2 (AI|GetBlackboard _returnvalue))
  (AI|Components|Blackboard|SetValueasVector _returnvalue_2 (Utilities|Name|MakeLiteralName "NoiseLocation") HitLocation)
  (AI|Components|Blackboard|SetValueasBool _returnvalue_2 (Utilities|Name|MakeLiteralName "soundPlay") false)
  (Utilities|FlowControl|Delay 0.2)
  (AI|Components|Blackboard|SetValueasBool _returnvalue_2 (Utilities|Name|MakeLiteralName "soundPlay") true)
  (Development|PrintString "AI Call")
  (Utilities|FlowControl|Delay 0.2))

(event EventBeginPlay
  (bind _returnvalue (Actor|GetActorOfClass "/Game/AIGhost/BP_Ghost.BP_Ghost_C"))
  (Variables|Default|SetGhostRef _returnvalue))

(fn ConstructionScript)