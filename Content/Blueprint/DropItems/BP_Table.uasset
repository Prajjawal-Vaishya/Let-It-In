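; BP_Table is a droppable table prop that makes noise when it hits something at speed.
; On a hit with mesh velocity above a threshold, it plays the Table_Drop sound at the impact point and calls AICall with that location, apparently to alert AI.
; A boolean gate with a short delay keeps repeated impacts from retriggering the sound and call.
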(event Collision|EventHit
  (params (MyComp :type Primitive%20Component%20Object%20Reference) (Other :type Actor%20Object%20Reference) (OtherComp :type Primitive%20Component%20Object%20Reference) (bSelfMoved :type Boolean) (HitLocation :type Vector :default "0, 0, 0") (HitNormal :type Vector :default "0, 0, 0") (NormalImpulse :type Vector :default "0, 0, 0") (Hit :type Hit%20Result%20Structure%20%28by%20ref%29))
  (if (and (Variables|Default|GetDelay) (> (Math|Vector|VectorLength (Transformation|GetComponentVelocity (Variables|Default|GetStaticMesh_0))) 1e+02))
    (Audio|PlaySoundatLocation "/Game/Sounds/Table_Drop.Table_Drop" HitLocation "0, 0, 0" 1.0 1.0 0.0 0 0 0 0)
    (CallFunction|AICall HitLocation)
    (Variables|Default|SetDelay false)
    (Utilities|FlowControl|Delay 2.0)
    (Variables|Default|SetDelay true)))

(fn ConstructionScript)