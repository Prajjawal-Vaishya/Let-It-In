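; BP_WaterTap is an interactable tap that plays water particles and sound and lures the ghost.
; Interact toggles it, with IsOn reading inverted: false while water runs.
; Turning it on writes the tap location to the ghost AI's blackboard as NoiseLocation and re-pulses soundPlay false then true after a short delay.
; A Ghost-tagged actor entering the box shuts off a running tap.
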(event OnComponentBeginOverlap(Box)
  (params (OverlappedComponent :type Primitive%20Component%20Object%20Reference) (OtherActor :type Actor%20Object%20Reference) (OtherComp :type Primitive%20Component%20Object%20Reference) (OtherBodyIndex :type Integer) (bFromSweep :type Boolean) (SweepResult :type Hit%20Result%20Structure%20%28by%20ref%29))
  (if (Actor|ActorHasTag OtherActor "Ghost")
    (if (not (Variables|Default|GetIsOn?))
      (Components|Activation|Deactivate (Variables|Default|GetNiagara))
      (Development|PrintString "TAP Off")
      (Components|Activation|Deactivate (Variables|Default|Gettap-water_Cue))
      (Variables|Default|SetIsOn? true))))

(event EventBeginPlay
  (bind _returnvalue (Actor|GetActorOfClass "/Game/AIGhost/BP_Ghost.BP_Ghost_C"))
  (Variables|Default|SetGhostRef _returnvalue))

(event EventInteract
  (bind _ghostref (Variables|Default|GetGhostRef))
  (bind _niagara (Variables|Default|GetNiagara))
  (bind _tap_water_cue (Variables|Default|Gettap-water_Cue))
  (bind _returnvalue (AI|GetAIController _ghostref))
  (bind _returnvalue_2 (AI|GetBlackboard _returnvalue))
  (if (Variables|Default|GetIsOn?)
    (Components|Activation|Activate _niagara false)
    (Development|PrintString "TAP ON")
    (Components|Activation|Activate _tap_water_cue false)
    (AI|Components|Blackboard|SetValueasVector _returnvalue_2 (Utilities|Name|MakeLiteralName "NoiseLocation") (Transformation|GetActorLocation))
    (AI|Components|Blackboard|SetValueasBool _returnvalue_2 (Utilities|Name|MakeLiteralName "soundPlay") false)
    (Utilities|FlowControl|Delay 0.2)
    (AI|Components|Blackboard|SetValueasBool _returnvalue_2 (Utilities|Name|MakeLiteralName "soundPlay") true)
    (Variables|Default|SetIsOn? false)
    (Development|PrintString "AI Call")
    (Utilities|FlowControl|Delay 0.2)
    (else
      (Components|Activation|Deactivate _niagara)
      (Development|PrintString "TAP Off")
      (Components|Activation|Deactivate _tap_water_cue)
      (Variables|Default|SetIsOn? true))))

(fn ConstructionScript)